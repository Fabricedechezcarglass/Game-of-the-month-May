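; An interactable push button actor that sets the Activé2 flag on the ThirdPersonCharacter when pressed with the Interagir input.
; Box overlap by that character opens and closes a Gate, so input only registers while the player is in range.
; A press plays a click sound, then one timeline lerps the button 10 units down along its relative Z and a second, played in reverse, returns it.
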(event OnComponentBeginOverlap(Box)
  (params (OverlappedComponent :type Primitive%20Component%20Object%20Reference) (OtherActor :type Actor%20Object%20Reference) (OtherComp :type Primitive%20Component%20Object%20Reference) (OtherBodyIndex :type Integer) (bFromSweep :type Boolean) (SweepResult :type Hit%20Result%20Structure%20%28by%20ref%29))
  (Utilities|Casting|CastToThirdPersonCharacter OtherActor)
  (Utilities|FlowControl|Gate true) ; enters at Open
)

(event OnComponentEndOverlap(Box)
  (params (OverlappedComponent :type Primitive%20Component%20Object%20Reference) (OtherActor :type Actor%20Object%20Reference) (OtherComp :type Primitive%20Component%20Object%20Reference) (OtherBodyIndex :type Integer))
  (Utilities|Casting|CastToThirdPersonCharacter OtherActor)
  (Utilities|FlowControl|Gate true) ; enters at Close
)

(event EventBeginPlay
  (bind _button (Variables|Default|Getbutton))
  (bind _returnvalue (Transformation|GetRelativeTransform _button))
  (Variables|Default|SetOut%20Position (Math|Transform|MakeTransform (.location _returnvalue) (.rotation _returnvalue) (.scale _returnvalue)))
  (Variables|Default|SetIn%20Position (Math|Transform|MakeTransform (- (.location _returnvalue) "0, 0,10.000000") (.rotation _returnvalue) (.scale _returnvalue)))
  (Input|EnableInput (Game|GetPlayerController 0)))

(event Input|ActionEvents|InputActionInteragir
  (params (Key :type Key%20Structure :default "None"))
  (:Pressed
    (Utilities|FlowControl|Gate true
      (:Exit
        (Audio|PlaySoundatLocation "/Engine/VREditor/Sounds/UI/Click_on_Button.Click_on_Button" (Transformation|GetActorLocation) "0, 0, 0" 1.0 1.0 0.0 0 0 0)
        (bind _asthird_person_character (Utilities|Casting|CastToThirdPersonCharacter (Game|GetPlayerCharacter 0)))
        (Variables|/Game/ThirdPersonBP/Blueprints/ThirdPersonCharacter.ThirdPersonCharacter_C|SetActivé2 _asthird_person_character true)
        (bind _button_in (Timeline|Timeline_0 PlayFromStart)
          (:Update
            (Transformation|SetRelativeTransform (Variables|Default|Getbutton) (Math|Transform|Lerp(Transform) (Variables|Default|GetOut%20Position) (Variables|Default|GetIn%20Position) _button_in) false false))
          (:Finished
            (bind _button_in_2 (Timeline|Timeline_1 ReverseFromEnd)
              (:Update
                (Transformation|SetRelativeTransform (Variables|Default|Getbutton) (Math|Transform|Lerp(Transform) (Variables|Default|GetOut%20Position) (Variables|Default|GetIn%20Position) _button_in_2) false false)))))))))

(fn ConstructionScript)
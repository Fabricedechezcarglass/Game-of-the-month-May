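; Destructible platform actor that wears down as it is stepped or jumped on, then disappears.
; Each begin overlap on its Box trigger increments a PlatformeJump counter, with no check on which actor overlaps.
; The first three hits swap the Platform material through three colour materials, and the fourth destroys the actor.
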(event OnComponentBeginOverlap(Box)
  (params (OverlappedComponent :type Primitive%20Component%20Object%20Reference) (OtherActor :type Actor%20Object%20Reference) (OtherComp :type Primitive%20Component%20Object%20Reference) (OtherBodyIndex :type Integer) (bFromSweep :type Boolean) (SweepResult :type Hit%20Result%20Structure%20%28by%20ref%29))
  (bind _output_get (Variables|Default|Setplatforme%20jump (+ (Variables|Default|Getplatforme%20jump) 1)))
  (switch int _output_get
    (:1
      (Rendering|Material|SetMaterial (Variables|Default|GetPlatform) 0 "/Game/Material/Couleur1.Couleur1"))
    (:2
      (Rendering|Material|SetMaterial (Variables|Default|GetPlatform) 0 "/Game/Material/Couleur2.Couleur2"))
    (:3
      (Rendering|Material|SetMaterial (Variables|Default|GetPlatform) 0 "/Game/Material/couleur3.couleur3"))
    (:4
      (Actor|DestroyActor))))

(fn ConstructionScript)